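; Player blueprint for a Geometry Dash-style auto-runner: a physics body that moves along Y at constant speed under strong custom downward acceleration.
; A box trace below it gates jumps, which reset vertical velocity, apply an impulse and roll the mesh another 90 degrees via timeline.
; Enhanced Input also toggles a pause menu widget with cursor and input mode switching.
; Any Box overlap prints "DEAD" and pauses the game.
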(event OnComponentBeginOverlap(Box)
  (params (OverlappedComponent :type Primitive%20Component%20Object%20Reference) (OtherActor :type Actor%20Object%20Reference) (OtherComp :type Primitive%20Component%20Object%20Reference) (OtherBodyIndex :type Integer) (bFromSweep :type Boolean) (SweepResult :type Hit%20Result%20Structure%20%28by%20ref%29))
  (Development|PrintString "DEAD")
  (Game|SetGamePaused true))

(event Input|EnhancedActionEvents|EnhancedInputActionIA_Jump
  (params (ActionValue :type Boolean) (ElapsedSeconds :type Float%20%28double-precision%29) (TriggeredSeconds :type Float%20%28double-precision%29) (InputAction :type Input%20Action%20Object%20Reference :default "/Game/IA_Jump.IA_Jump"))
  (bind _collision (Variables|Default|GetCollision))
  (bind _returnvalue (Transformation|GetWorldLocation _collision))
  (bind _returnvalue_2 (- _returnvalue "0.000000,0.000000,50.000000"))
  (bind _returnvalue_3 (Collision|BoxTraceByChannel _returnvalue_2 _returnvalue_2 "40.000000,40.000000,10.000000" "0, 0, 0" "TraceTypeQuery1" false 0 "ForOneFrame"))
  (if _returnvalue_3
    (bind _returnvalue_4 (Physics|GetPhysicsLinearVelocity (Variables|Default|GetCollision) "None"))
    (Physics|SetPhysicsLinearVelocity (Variables|Default|GetCollision) (Math|Vector|MakeVector (.x _returnvalue_4) (.y _returnvalue_4) 0.0) false "None")
    (Physics|AddImpulse (Variables|Default|GetCollision) (Math|Vector|MakeVector 0.0 0.0 (Variables|Default|GetJumpVelocity)) "None" true)
    (Variables|Default|SetTargetRotation (+ (Variables|Default|GetTargetRotation) 9e+01))
    (Components|Timeline|SetPlayRate (Variables|Default|GetTimeline) (/ 1.0 (Variables|Default|GetTimeRotation)))
    (bind _newtrack_0 (Timeline|Timeline PlayFromStart)
      (:Update
        (Transformation|SetRelativeRotation (Variables|Default|GetSM_Player) (Math|Rotator|MakeRotator (Math|Float|Lerp (- (Variables|Default|GetTargetRotation) 9e+01) (Variables|Default|GetTargetRotation) _newtrack_0) 0.0 0.0) false false)))))

(event Input|EnhancedActionEvents|EnhancedInputActionIA_Pause
  (params (ActionValue :type Boolean) (ElapsedSeconds :type Float%20%28double-precision%29) (TriggeredSeconds :type Float%20%28double-precision%29) (InputAction :type Input%20Action%20Object%20Reference :default "/Game/IA_Pause.IA_Pause"))
  (bind _returnvalue (Game|GetPlayerController 0))
  (bind _returnvalue_2 (Game|GetPlayerController 0))
  (:Started
    (if (Game|IsGamePaused)
      (Game|SetGamePaused false)
      (Input|SetInputModeGameOnly _returnvalue false)
      (Variables|/Script/Engine.PlayerController|SetbShowMouseCursor _returnvalue false)
      (Widget|RemovefromParent (Variables|Default|GetPauseMenuRef))
      (else
        (Game|SetGamePaused true)
        (Variables|Default|GetPauseMenuRef
          (:then
            _)
          (:else
            (bind _returnvalue_3 (UserInterface|CreateWidget "/Game/WG_PauseMenu.WG_PauseMenu_C"))
            (Variables|Default|SetPauseMenuRef _returnvalue_3)))
        (UserInterface|Viewport|AddtoViewport (Variables|Default|GetPauseMenuRef) 0)
        (Input|SetInputModeGameandUI _returnvalue_2 (Variables|Default|GetPauseMenuRef) "DoNotLock" false false)
        (Variables|/Script/Engine.PlayerController|SetbShowMouseCursor _returnvalue_2 true)))))

(event EventBeginPlay
  (Input|AddMappingContext (PlayerController|LocalPlayerSubsystems|GetEnhancedInputLocalPlayerSubsystem (Game|GetPlayerController 0)) "/Game/IMC_Player.IMC_Player" 0 "(bIgnoreAllPressedKeysUntilRelease=True,bForceImmediately=False,bNotifyUserSettings=False)"))

(event EventTick
  (params (DeltaSeconds :type Float%20%28single-precision%29))
  (bind _collision (Variables|Default|GetCollision))
  (Physics|AddForce (Variables|Default|GetCollision) "0.000000,0.000000,-9404.000000" "None" true)
  (bind _returnvalue (Physics|GetPhysicsLinearVelocity _collision "None"))
  (Physics|SetPhysicsLinearVelocity _collision (Math|Vector|MakeVector 0.0 (Variables|Default|GetPlayerSpeed) (.z _returnvalue)) false "None"))

(fn ConstructionScript)